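; BP_Enemy2 is a flying enemy that patrols vertically and instantly kills the player on contact.
; BeginPlay sets flying movement and bounds 300 units above and below the start height, then starts the self-repeating Roam event.
; Roam flips direction past either bound, adding movement input every 0.1 seconds.
; Sphere overlap with BP_Player zeroes Health, shows GameOver with UI-only input, and hides the player with collision disabled.
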(event OnComponentBeginOverlap(Sphere)
  (params (OverlappedComponent :type Primitive%20Component%20Object%20Reference) (OtherActor :type Actor%20Object%20Reference) (OtherComp :type Primitive%20Component%20Object%20Reference) (OtherBodyIndex :type Integer) (bFromSweep :type Boolean) (SweepResult :type Hit%20Result%20Structure%20%28by%20ref%29))
  (bind _returnvalue (Game|GetPlayerController 0))
  (bind _asbp_player (Utilities|Casting|CastToBP_Player OtherActor))
  (Variables|/Game/Blueprints/BP_Player.BP_Player_C|Sethealth _asbp_player 0.0)
  (bind _returnvalue_2 (UserInterface|CreateWidget "/Game/Blueprints/UI/GameOver.GameOver_C"))
  (UserInterface|Viewport|AddtoViewport _returnvalue_2 0)
  (Input|SetIgnoreMoveInput _returnvalue true)
  (Input|SetInputModeUIOnly _returnvalue 0 "DoNotLock" false)
  (Variables|/Script/Engine.PlayerController|SetbShowMouseCursor _returnvalue true)
  (Collision|SetActorEnableCollision _asbp_player false)
  (Rendering|SetActorHiddenInGame _asbp_player true))

(event Custom|Roam
  (bind _returnvalue (Transformation|GetActorLocation))
  (if (> (Variables|Default|Getmin_z) (.z _returnvalue))
    (Variables|Default|Setz 1.0)
    (elif (> (.z _returnvalue) (Variables|Default|Getmax_z))
      (Variables|Default|Setz -1.0)))
  (Pawn|Input|AddMovementInput (Math|Vector|MakeVector 0.0 0.0 (Variables|Default|Getz)) 1.0 false)
  (Utilities|FlowControl|Delay 0.1)
  (CallFunction|Roam))

(event EventBeginPlay
  (Variables|Default|Setz (.z (Transformation|GetActorLocation)))
  (Variables|Default|Setmax_z (+ 3e+02 (Variables|Default|Getz)))
  (Variables|Default|Setmin_z (+ -3e+02 (Variables|Default|Getz)))
  (Pawn|Components|CharacterMovement|SetMovementMode (Variables|Character|GetCharacterMovement) "MOVE_Flying" 0)
  (Variables|Default|Setz -1.0)
  (CallFunction|Roam))

(fn ConstructionScript)