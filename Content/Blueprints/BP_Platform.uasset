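; BP_Platform is a 2D sprite platform that cyclically disappears and reappears.
; From BeginPlay, the Disappear event alternates on fixed delays between hiding with actor collision off and showing with collision on, then calls itself to loop indefinitely.
; Hiding targets the Box and propagates to its children, while showing unhides only the PaperSprite, so the Box itself stays hidden after the first cycle.
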(event Custom|Disappear
  (Utilities|FlowControl|Delay 3.0)
  (Development|SetHiddeninGame (Variables|Default|GetBox) true true)
  (Collision|SetActorEnableCollision false)
  (Utilities|FlowControl|Delay 3.0)
  (Development|SetHiddeninGame (Variables|Default|GetPaperSprite) false false)
  (Collision|SetActorEnableCollision true)
  (CallFunction|Disappear))

(event EventBeginPlay
  (CallFunction|Disappear))

(event Collision|EventActorBeginOverlap
  (params (OtherActor :type Actor%20Object%20Reference)))

(event EventTick
  (params (DeltaSeconds :type Float%20%28single-precision%29)))

(fn ConstructionScript)